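; BP_EnemySon_1 is a child enemy Blueprint that sets up side-to-side movement along the world Y axis.
; On BeginPlay it runs the parent logic, then seeds MovementVector from the actor's right vector.
; CheckLimits flips the vector's Y and zeroes X and Z whenever the actor is outside LimitLeftY or LimitRightY.
; Neither the movement itself nor the call to CheckLimits appears in this Blueprint.
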(event EventBeginPlay
  (|CallParentFunction)
  (Variables|Default|SetMovementVector (Transformation|GetActorRightVector)))

(event Collision|EventActorBeginOverlap
  (params (OtherActor :type Actor%20Object%20Reference))
  (|CallParentFunction OtherActor) ; This node is disabled and will not be called.\nDrag off pins to build functionality.
)

(event EventTick
  (params (DeltaSeconds :type Float%20%28single-precision%29))
  (|CallParentFunction DeltaSeconds) ; This node is disabled and will not be called.\nDrag off pins to build functionality.
)

(fn ConstructionScript
  (|CallParentFunction))

(fn CheckLimits
  (bind _returnvalue (Transformation|GetActorLocation))
  (bind _y (Math|Vector|BreakVector _returnvalue))
  (if (or (> _y (Variables|Default|GetLimitRightY)) (< _y (Variables|Default|GetLimitLeftY)))
    (Variables|Default|SetMovementVector (* (Variables|Default|GetMovementVector) "0.000000,-1.000000,0.000000"))))