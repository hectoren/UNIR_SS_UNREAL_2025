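; Enemy spawner actor that creates a random enemy at a regular interval.
; On BeginPlay a looping timer starts calling SpawnEnemy, and the BP_SS_Game_Mode reference is cached.
; The enemy class is picked at random within the game mode's Level, clamped by MaxNumEnemies, choosing between BP_EnemyBase and BP_EnemySon_1.
; Spawn location comes from a random pick among its own scene components tagged SpawnPoint.
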(event Custom|Spawn
  (CallFunction|SpawnEnemy))

(event EventBeginPlay
  (Utilities|Time|SetTimerbyEvent (delegate Custom|Spawn) (Variables|Default|GetSpawnTime) true)
  (bind _asbp_ss_game_mode (Utilities|Casting|CastToBP_SS_Game_Mode (Game|GetGameMode)))
  (Variables|Default|SetSSGameMode _asbp_ss_game_mode))

(event Collision|EventActorBeginOverlap
  (params (OtherActor :type Actor%20Object%20Reference)))

(event EventTick
  (params (DeltaSeconds :type Float%20%28single-precision%29)))

(fn ConstructionScript)

(fn SpawnEnemy
  (bind _returnvalue (Actor|GetComponentsbyTag "/Script/Engine.SceneComponent" "SpawnPoint"))
  (bind _class (CallFunction|GetClasstoSpawn (Math|Random|RandomInteger (Variables|/Game/BP_SS_Game_Mode.BP_SS_Game_Mode_C|GetLevel (Variables|Default|GetSSGameMode)))))
  (bind _returnvalue_2 (Game|SpawnActorfromClass _class (Transformation|GetWorldTransform (Utilities|Array|Get(acopy) _returnvalue (Math|Random|RandomInteger (Utilities|Array|Length _returnvalue)))) "Undefined" "MultiplyWithRoot" 0 0))
  (bind _asbp_enemy_base (Utilities|Casting|CastToBP_EnemyBase _returnvalue_2))
  (return _asbp_enemy_base))

(fn GetClasstoSpawn
  (params (Type :type Integer))
  (return (Utilities|Select :Index (Math|Integer|Clamp(Integer) Type 0 (- (Variables|Default|GetMaxNumEnemies) 1)) :Option%200 "/Game/Enemies/BP_EnemyBase.BP_EnemyBase_C" :Option%201 "/Game/Enemies/BP_EnemySon_1.BP_EnemySon_1_C")))