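; BP_Enemy_Ammo is an enemy projectile that flies straight along its forward vector at a set Speed.
; Tick moves it each frame by offsetting its location without sweeping.
; Overlapping an actor tagged Player or Edge spawns a SimpleExplosion particle system at its location, then destroys it after a short delay.
; It applies no damage itself.
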(event EventBeginPlay)

(event Collision|EventActorBeginOverlap
  (params (OtherActor :type Actor%20Object%20Reference))
  (bind _tags (Variables|/Script/Engine.Actor|GetTags OtherActor))
  (if (or (Utilities|Array|ContainsItem _tags "Player") (Utilities|Array|ContainsItem _tags "Edge"))
    (Niagara|SpawnSystematLocation "/Niagara/DefaultAssets/Templates/Systems/SimpleExplosion.SimpleExplosion" (Transformation|GetActorLocation))
    (Utilities|FlowControl|Delay 0.2)
    (Actor|DestroyActor)))

(event EventTick
  (params (DeltaSeconds :type Float%20%28single-precision%29))
  (Transformation|SetActorLocation (+ (Transformation|GetActorLocation) (* (Transformation|GetActorForwardVector) (* DeltaSeconds (Variables|Default|GetSpeed)))) false false))

(fn ConstructionScript)